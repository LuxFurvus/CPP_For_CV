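; Player character Blueprint that maps keyboard input to base linking, build mode, turret color selection and turret building.
; Number keys pick one of four colors, and R builds from turret traits, with a server event spawning BP_Turrel at a valid build place.
; Debug keys change base health and kill turrets through server calls.
; Most gameplay functions are called here but defined outside these graphs.
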(event Custom|MakeTur_SERVER
  (params (Spawn%20Transform%20Location :type Vector) (TurretTraits :type Turret%20Traits%20Structure) (Owner :type Actor%20Object%20Reference))
  ;[1 1 1] Comment
  (Game|SpawnActorfromClass "/Game/ASSETS/BP_Turrel.BP_Turrel_C" (Math|Transform|MakeTransform Spawn%20Transform%20Location "0, 0, 0" "1.000000,1.000000,1.000000") "AlwaysSpawn" "MultiplyWithRoot" Owner TurretTraits 0))

(event Input|KeyboardEvents|B
  (params (Key :type Key%20Structure :default "None"))
  ;[0 0 0] READY
  (:Pressed
    (Class|CPlayerCharacter|OpenBuildMode)))

(event Input|KeyboardEvents|R
  (params (Key :type Key%20Structure :default "None"))
  (bind _dt_turrettraits (Variables|Default|GetDT_TurretTraits))
  ;[0 0 0] READY
  (:Pressed
    (Class|CPlayerCharacter|BuildTurret _dt_turrettraits)
    ;[1 1 1] Comment
    (Class|CPlayerCharacter|BuildTurretSERVER _dt_turrettraits)
    (if (and (Variables|Default|GetHasPlaceToBuild) (Variables|Default|GetCanBuildTurret))
      (CallFunction|MakeTurSERVER (Variables|Default|GetPlaceToBuild) (Variables|Default|GetTurretTraits) self))))

(event Input|KeyboardEvents|ShiftR
  (params (Key :type Key%20Structure :default "None"))
  ;[0 0 0] READY
  (:Pressed
    (Class|CPlayerCharacter|KillTurretSERVER 10)))

(event Input|KeyboardEvents|Q
  (params (Key :type Key%20Structure :default "None"))
  ;[0 0 0] READY
  (:Pressed
    (Class|CPlayerCharacter|SetPlayerBaseLinkCLIENT)))

(event Input|KeyboardEvents|4
  (params (Key :type Key%20Structure :default "None"))
  ;[0 0 0] READY
  (:Pressed
    (Class|CPlayerCharacter|SelectTurretColor (Utilities|Name|MakeLiteralName "Red"))))

(event Input|KeyboardEvents|ShiftE
  (params (Key :type Key%20Structure :default "None"))
  ;[0 0 0] READY
  (:Pressed
    (Class|CPlayerCharacter|TESTChangeBaseHealthSERVER 1e+01)))

(event Input|KeyboardEvents|E
  (params (Key :type Key%20Structure :default "None"))
  ;[0 0 0] READY
  (:Pressed
    (Class|CPlayerCharacter|TESTChangeBaseHealthSERVER -1e+01)))

(event Input|KeyboardEvents|3
  (params (Key :type Key%20Structure :default "None"))
  ;[0 0 0] READY
  (:Pressed
    (Class|CPlayerCharacter|SelectTurretColor (Utilities|Name|MakeLiteralName "Orange"))))

(event Input|KeyboardEvents|1
  (params (Key :type Key%20Structure :default "None"))
  ;[0 0 0] READY
  (:Pressed
    (Class|CPlayerCharacter|SelectTurretColor (Utilities|Name|MakeLiteralName "Violet"))))

(event Input|KeyboardEvents|2
  (params (Key :type Key%20Structure :default "None"))
  ;[0 0 0] READY
  (:Pressed
    (Class|CPlayerCharacter|SelectTurretColor (Utilities|Name|MakeLiteralName "Blue"))))

(fn ConstructionScript)
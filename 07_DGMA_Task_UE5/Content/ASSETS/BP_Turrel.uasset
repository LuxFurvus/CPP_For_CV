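; BP_Turrel is an auto-firing turret that attacks actors implementing BPI_TurretMarker with a different owner.
; Each tick a server event sphere-traces for targets, damages the nearest found so far per qualifying hit, and calls a multicast that aims the gun and spawns a delayed Niagara beam.
; Damage lowers Health, whose OnRep updates a dynamic material tinted by TurretTraits and, at zero, sets IsDead and hides the gun.
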(event Custom|CustomEvent
  (bind _turretbase (Variables|Default|GetTurretBase))
  (bind _returnvalue (Rendering|Material|CreateDynamicMaterialInstance _turretbase 0 (Rendering|Material|GetMaterial _turretbase 0) "None" :!class /Script/Engine.PrimitiveComponent))
  (bind _output_get (Variables|Default|SetMID_Turret _returnvalue))
  (Rendering|Material|SetMaterial (Variables|Default|GetTurretGun) 0 _output_get)
  (Rendering|Material|SetVectorParameterValue _output_get "COLOR" (Utilities|Struct|Break_TurretTraits (Variables|Default|GetTurretTraits)) :!class /Script/Engine.MaterialInstanceDynamic))

(event Custom|EEEE
  (CallFunction|CustomEvent))

(event Custom|ShootBP_MULTI
  (params (New%20Rotation%20Z%20%28Yaw%29 :type Float%20%28single-precision%29) (Param :type Vector))
  (Transformation|SetWorldRotation (Variables|Default|GetTurretGun) (Math|Rotator|MakeRotator 0.0 0.0 New%20Rotation%20Z%20%28Yaw%29) false false)
  (Utilities|FlowControl|Delay (Variables|Default|GetReactionDelay))
  (bind _returnvalue (Niagara|SpawnSystematLocation "/Game/ASSETS/VFX/NS_GunTrailFire.NS_GunTrailFire" "0, 0, 0"))
  (Effects|Components|ParticleSystem|SetVectorParameter _returnvalue "BeamStart" (Transformation|GetWorldLocation (Variables|Default|GetFirePoint)))
  (Effects|Components|ParticleSystem|SetVectorParameter _returnvalue "BeamEnd" Param)
  (Effects|Components|ParticleSystem|SetFloatParameter _returnvalue "Lifetime" 0.5))

(event Custom|ShootBP_SERVER
  (bind _returnvalue (Transformation|GetActorLocation))
  (if (not (Variables|Default|GetIsDead))
    (Utilities|Array|Clear (Variables|Default|GetTargets))
    (bind _outhits (Collision|MultiSphereTraceByChannel _returnvalue (+ _returnvalue 0.01) (Variables|Default|GetRadius) "TraceTypeQuery1" false 0 "None"))
    (for _array_element _outhits
      (if (and (Utilities|DoesObjectImplementInterface (.HitActor (Collision|BreakHitResult _array_element)) "/Game/ASSETS/BPI_TurretMarker.BPI_TurretMarker_C") (!= (Components|GetOwner) (Components|GetOwner (.HitActor (Collision|BreakHitResult _array_element)))))
        (Utilities|Array|AddUnique (Variables|Default|GetTargets) (.HitActor (Collision|BreakHitResult _array_element)))
        (bind _output_get (Variables|Default|SetTarget (.ReturnValue (Actor|FindNearestActor (Transformation|GetWorldLocation (Variables|Default|GetTurretBase)) (Variables|Default|GetTargets)))))
        (Game|Damage|ApplyDamage _output_get (/ (Utilities|Struct|Break_TurretTraits (Variables|Default|GetTurretTraits)) 1e+02) 0 0)
        (CallFunction|ShootBPMULTI (+ (.yaw (Math|Conversions|RotationFromXVector (Math|Vector|GetRightVector (Math|Rotator|FindLookatRotation (Transformation|GetActorLocation) (Transformation|GetActorLocation _output_get))))) 1.8e+02) (Transformation|GetActorLocation _output_get))))))

(event EventBeginPlay
  (Variables|Default|SetHealth (Utilities|Struct|Break_TurretTraits (Variables|Default|GetTurretTraits)))
  (CallFunction|EEEE))

(event EventTick
  (params (DeltaSeconds :type Float%20%28single-precision%29))
  (Development|PrintString (Utilities|String|Append (Utilities|GetDisplayName self) " = " (Utilities|String|ToString(Float) (Variables|Default|GetHealth)) " = " (Utilities|GetDisplayName (Variables|Default|GetTarget))) true false "(R=0.000000,G=0.660000,B=1.000000,A=1.000000)" 0.0)
  (CallFunction|ShootBPSERVER))

(event Game|Damage|EventAnyDamage
  (params (Damage :type Float%20%28single-precision%29) (DamageType :type Damage%20Type%20Object%20Reference) (InstigatedBy :type Controller%20Object%20Reference) (DamageCauser :type Actor%20Object%20Reference))
  (Variables|Default|SetHealth (Math|Float|Clamp(Float) (- (Variables|Default|GetHealth) Damage) 0.0 (Utilities|Struct|Break_TurretTraits (Variables|Default|GetTurretTraits)))))

(fn ConstructionScript)

(fn OnRepHealth
  (bind _mid_turret (Variables|Default|GetMID_Turret)
    (:then
      (Rendering|Material|SetScalarParameterValue _mid_turret "Health" (/ (Variables|Default|GetHealth) (Utilities|Struct|Break_TurretTraits (Variables|Default|GetTurretTraits))) :!class /Script/Engine.MaterialInstanceDynamic))
    (:else
      _))
  (if (<= (Variables|Default|GetHealth) 0.0)
    (Variables|Default|SetIsDead true)
    (Rendering|SetVisibility (Variables|Default|GetTurretGun) false false)))